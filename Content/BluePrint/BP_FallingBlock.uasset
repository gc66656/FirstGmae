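; Falling Tetris-style piece whose construction script arranges four cubes into one of seven random colored shapes.
; Player input moves or rotates it, reverting if box overlaps hit WorldStatic, and speeds descent through global time dilation.
; A looping timer steps it down until line traces detect support.
; It then spawns BP_SingleBlock per child component, triggers CheckLines on CheckLinesActor, spawns the next piece and destroys itself.
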(event `InputAction|RotateBlock`
  (params (Key :type "Key Structure"))
  (:`Pressed`
    (`self.K2_AddActorLocalRotation` (struct :`Roll` 90.0))
    (for _array_element (`self.K2_GetComponentsByClass` "/Script/Engine.StaticMeshComponent")
      (bind (_outactors _returnvalue) (`KismetSystemLibrary.BoxOverlapActors` (`SceneComponent.K2_GetComponentLocation` _array_element) (15.0 15.0 15.0) (`|MakeArray` "ObjectTypeQuery1" :!type "EObjectTypeQuery Enum")))
      (if _returnvalue
        (`self.K2_AddActorLocalRotation` (struct :`Roll` -90.0))
        (break)))))

(event `InputAction|MoveBlockLeft`
  (params (Key :type "Key Structure"))
  (:`Pressed`
    (`self.Try Later Movement` -50.0)))

(event `InputAction|MoveBlockRight`
  (params (Key :type "Key Structure"))
  (:`Pressed`
    (`self.Try Later Movement` 50.0)))

(event `InputAction|SpeedBlockDescent`
  (params (Key :type "Key Structure"))
  (:`Pressed`
    (`GameplayStatics.SetGlobalTimeDilation` 5.0))
  (:`Released`
    (`GameplayStatics.SetGlobalTimeDilation` 1.0)))

(event `self.ReceiveBeginPlay`
  (bind _returnvalue (`KismetSystemLibrary.K2_SetTimerDelegate` (delegate `DropBlock`) (`self.DropSpeed`) true))
  (set `self.BlockDroppingTimer` _returnvalue))

(event `DropBlock`
  (set `self.ShouldDrop?` true)
  (for _array_element (`SceneComponent.GetChildrenComponents` (`self.DefaultSceneRoot`) false)
    (bind _returnvalue (`SceneComponent.K2_GetComponentLocation` _array_element))
    (bind (_outhit _returnvalue_2) (`KismetSystemLibrary.LineTraceSingleForObjects` _returnvalue (- _returnvalue (0.0 0.0 50.0)) (`|MakeArray` "ObjectTypeQuery1" :!type "EObjectTypeQuery Enum")))
    (if _returnvalue_2
      (`/Engine/EditorBlueprintResources/StandardMacros.DoOnce` false
        (:`Completed`
          (set `self.ShouldDrop?` false)
          (`KismetSystemLibrary.K2_ClearAndInvalidateTimerHandle` (`self.BlockDroppingTimer`))))))
  (if (`self.ShouldDrop?`)
    (`self.K2_AddActorWorldOffset` (0.0 0.0 -50.0))
    (else
      (for _array_element_2 (`SceneComponent.GetChildrenComponents` (`self.DefaultSceneRoot`) false)
        (`|SpawnActorFromClass` "/Game/BluePrint/BP_SingleBlock.BP_SingleBlock_C" (`KismetMathLibrary.MakeTransform` (`SceneComponent.K2_GetComponentLocation` _array_element_2)) "Undefined" "OverrideRootScale" null (`self.BlockColor`) null))
      (`/Game/BluePrint/BP_CheckLine.CheckLines` (`self.CheckLinesActor`))
      (`|SpawnActorFromClass` "BP_FallingBlock_C" (`KismetMathLibrary.MakeTransform` (0.0 25.0 1000.0)) "Undefined" "OverrideRootScale" null (`self.CheckLinesActor`) null)
      (`self.K2_DestroyActor`))))

(fn `Try Later Movement`
  (params (MoveAmount :type "Float (double-precision)"))
  (`self.K2_AddActorWorldOffset` (`KismetMathLibrary.MakeVector` 0.0 MoveAmount))
  (for _array_element (`self.K2_GetComponentsByClass` "/Script/Engine.StaticMeshComponent")
    (bind (_outactors _returnvalue) (`KismetSystemLibrary.BoxOverlapActors` (`SceneComponent.K2_GetComponentLocation` _array_element) (15.0 15.0 15.0) (`|MakeArray` "ObjectTypeQuery1" :!type "EObjectTypeQuery Enum")))
    (if _returnvalue
      (`self.K2_AddActorWorldOffset` (`KismetMathLibrary.MakeVector` 0.0 (- 0.0 (`local.MoveAmount`))))
      (break))))

(fn `UserConstructionScript`
  (switch `int` (`KismetMathLibrary.RandomIntegerInRange` 0 6)
    (:`Default`
      ;[1 1 1] 创建 方
      (`SceneComponent.K2_AddLocalOffset` (`self.cbue2`) (0.0 0.0 50.0) false false)
      (`SceneComponent.K2_AddLocalOffset` (`self.cbue3`) (0.0 50.0 0.0) false false)
      (`SceneComponent.K2_AddLocalOffset` (`self.cbue4`) (0.0 50.0 50.0) false false)
      (set `self.BlockColor` (struct :`R` 0.085431 :`G` 1.0 :`A` 1.0)))
    (:`0`
      ;[1 1 1] 创建长条
      (`SceneComponent.K2_AddLocalOffset` (`self.cbue2`) (0.0 0.0 50.0) false false)
      (`SceneComponent.K2_AddLocalOffset` (`self.cbue3`) (0.0 0.0 100.0) false false)
      (`SceneComponent.K2_AddLocalOffset` (`self.cbue4`) (0.0 0.0 150.0) false false)
      (set `self.BlockColor` (struct :`R` 1.0 :`G` 0.839427 :`A` 1.0)))
    (:`1`
      ;[1 1 1] 创建L
      (`SceneComponent.K2_AddLocalOffset` (`self.cbue2`) (0.0 0.0 50.0) false false)
      (`SceneComponent.K2_AddLocalOffset` (`self.cbue3`) (0.0 0.0 100.0) false false)
      (`SceneComponent.K2_AddLocalOffset` (`self.cbue4`) (0.0 50.0 0.0) false false)
      (set `self.BlockColor` (struct :`R` 1.0 :`B` 0.00718 :`A` 1.0)))
    (:`2`
      ;[1 1 1] 反向L
      (`SceneComponent.K2_AddLocalOffset` (`self.cbue2`) (0.0 0.0 50.0) false false)
      (`SceneComponent.K2_AddLocalOffset` (`self.cbue3`) (0.0 0.0 100.0) false false)
      (`SceneComponent.K2_AddLocalOffset` (`self.cbue4`) (0.0 -50.0 0.0) false false)
      (set `self.BlockColor` (struct :`R` 1.0 :`G` 0.254883 :`A` 1.0)))
    (:`3`
      ;[1 1 1] 创建S
      (`SceneComponent.K2_AddLocalOffset` (`self.cbue2`) (0.0 0.0 50.0) false false)
      (`SceneComponent.K2_AddLocalOffset` (`self.cbue3`) (0.0 50.0 50.0) false false)
      (`SceneComponent.K2_AddLocalOffset` (`self.cbue4`) (0.0 50.0 100.0) false false)
      (set `self.BlockColor` (struct :`R` 1.0 :`B` 0.656677 :`A` 1.0)))
    (:`4`
      ;[1 1 1] 创建反S
      (`SceneComponent.K2_AddLocalOffset` (`self.cbue2`) (0.0 0.0 50.0) false false)
      (`SceneComponent.K2_AddLocalOffset` (`self.cbue3`) (0.0 -50.0 50.0) false false)
      (`SceneComponent.K2_AddLocalOffset` (`self.cbue4`) (0.0 -50.0 100.0) false false)
      (set `self.BlockColor` (struct :`R` 0.035364 :`B` 1.0 :`A` 1.0)))
    (:`5`
      ;[1 1 1] 创建T
      (`SceneComponent.K2_AddLocalOffset` (`self.cbue2`) (0.0 -50.0 0.0) false false)
      (`SceneComponent.K2_AddLocalOffset` (`self.cbue3`) (0.0 0.0 50.0) false false)
      (`SceneComponent.K2_AddLocalOffset` (`self.cbue4`) (0.0 50.0 0.0) false false)
      (set `self.BlockColor` (struct :`G` 1.0 :`B` 1.0 :`A` 1.0))))
  (`MeshComponent.SetVectorParameterValueOnMaterials` (`self.cbue1`) "GlowColor" (`KismetMathLibrary.Conv_LinearColorToVector` (`self.BlockColor`)))
  (`MeshComponent.SetVectorParameterValueOnMaterials` (`self.cbue2`) "GlowColor" (`KismetMathLibrary.Conv_LinearColorToVector` (`self.BlockColor`)))
  (`MeshComponent.SetVectorParameterValueOnMaterials` (`self.cbue3`) "GlowColor" (`KismetMathLibrary.Conv_LinearColorToVector` (`self.BlockColor`)))
  (`MeshComponent.SetVectorParameterValueOnMaterials` (`self.cbue4`) "GlowColor" (`KismetMathLibrary.Conv_LinearColorToVector` (`self.BlockColor`))))