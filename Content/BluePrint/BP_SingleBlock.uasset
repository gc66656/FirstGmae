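; BP_SingleBlock is a single block actor with a tinted glow and smoothed vertical movement.
; On BeginPlay it pushes BlockColor into the mesh materials' GlowColor parameter and stores its current height as TargetZ.
; Each Tick it lerps its Z a fixed fraction toward TargetZ, keeping X and Y, so the easing depends on frame rate.
; Nothing in this graph changes TargetZ after initialization.
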(event `self.ReceiveBeginPlay`
  (bind (_returnvalue_x _returnvalue_y _returnvalue_z) (`KismetMathLibrary.BreakVector` (`self.K2_GetActorLocation`)))
  (`MeshComponent.SetVectorParameterValueOnMaterials` (`self.StaticMesh`) "GlowColor" (`KismetMathLibrary.Conv_LinearColorToVector` (`self.BlockColor`)))
  (set `self.TargetZ` _returnvalue_z))

(event `self.ReceiveTick`
  (params (DeltaSeconds :type "Float (single-precision)"))
  (bind (_returnvalue_x _returnvalue_y _returnvalue_z) (`KismetMathLibrary.BreakVector` (`self.K2_GetActorLocation`)))
  (bind (_returnvalue_x_2 _returnvalue_y_2 _returnvalue_z_2) (`KismetMathLibrary.BreakVector` (`self.K2_GetActorLocation`)))
  (if (not (`KismetMathLibrary.NearlyEqual_FloatFloat` (`self.TargetZ`) _returnvalue_z_2))
    (`self.K2_SetActorLocation` (`KismetMathLibrary.MakeVector` _returnvalue_x _returnvalue_y (`KismetMathLibrary.Lerp` _returnvalue_z (`self.TargetZ`) 0.05)))))

(fn `UserConstructionScript`)