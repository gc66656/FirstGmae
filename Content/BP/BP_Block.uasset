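; BP_Block is a tetromino piece actor that takes a random shape when constructed.
; Its Construction Script switches on a random integer and offsets four cube components on a 50-unit grid in the local YZ plane.
; RandomInteger(6) yields only 0–5, so the seventh case, a T shape mislabeled as an S, is never chosen.
; The event graph holds only disabled stubs, so the Blueprint has no movement or gameplay logic.
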(fn `UserConstructionScript`
  (switch `int` (`KismetMathLibrary.RandomInteger` 6)
    (:`0`
      ;[1 1 1] I
      (`SceneComponent.K2_AddLocalOffset` (`self.Cube1`) (0.0 0.0 0.0) false false)
      (`SceneComponent.K2_AddLocalOffset` (`self.Cube2`) (0.0 50.0 0.0) false false)
      (`SceneComponent.K2_AddLocalOffset` (`self.Cube3`) (0.0 100.0 0.0) false false)
      (`SceneComponent.K2_AddLocalOffset` (`self.Cube4`) (0.0 150.0 0.0) false false))
    (:`1`
      ;[1 1 1] L左
      (`SceneComponent.K2_AddLocalOffset` (`self.Cube1`) (0.0 0.0 0.0) false false)
      (`SceneComponent.K2_AddLocalOffset` (`self.Cube2`) (0.0 0.0 50.0) false false)
      (`SceneComponent.K2_AddLocalOffset` (`self.Cube3`) (0.0 50.0 0.0) false false)
      (`SceneComponent.K2_AddLocalOffset` (`self.Cube4`) (0.0 100.0 0.0) false false))
    (:`2`
      ;[1 1 1] L右
      (`SceneComponent.K2_AddLocalOffset` (`self.Cube1`) (0.0 0.0 0.0) false false)
      (`SceneComponent.K2_AddLocalOffset` (`self.Cube2`) (0.0 50.0 0.0) false false)
      (`SceneComponent.K2_AddLocalOffset` (`self.Cube3`) (0.0 100.0 0.0) false false)
      (`SceneComponent.K2_AddLocalOffset` (`self.Cube4`) (0.0 100.0 50.0) false false))
    (:`3`
      ;[1 1 1] 口
      (`SceneComponent.K2_AddLocalOffset` (`self.Cube1`) (0.0 0.0 0.0) false false)
      (`SceneComponent.K2_AddLocalOffset` (`self.Cube2`) (0.0 50.0 0.0) false false)
      (`SceneComponent.K2_AddLocalOffset` (`self.Cube3`) (0.0 50.0 50.0) false false)
      (`SceneComponent.K2_AddLocalOffset` (`self.Cube4`) (0.0 0.0 50.0) false false))
    (:`4`
      ;[1 1 1] S左
      (`SceneComponent.K2_AddLocalOffset` (`self.Cube1`) (0.0 0.0 0.0) false false)
      (`SceneComponent.K2_AddLocalOffset` (`self.Cube2`) (0.0 50.0 0.0) false false)
      (`SceneComponent.K2_AddLocalOffset` (`self.Cube3`) (0.0 50.0 50.0) false false)
      (`SceneComponent.K2_AddLocalOffset` (`self.Cube4`) (0.0 100.0 50.0) false false))
    (:`5`
      ;[1 1 1] S右
      (`SceneComponent.K2_AddLocalOffset` (`self.Cube1`) (0.0 0.0 0.0) false false)
      (`SceneComponent.K2_AddLocalOffset` (`self.Cube2`) (0.0 50.0 0.0) false false)
      (`SceneComponent.K2_AddLocalOffset` (`self.Cube3`) (0.0 0.0 50.0) false false)
      (`SceneComponent.K2_AddLocalOffset` (`self.Cube4`) (0.0 -50.0 50.0) false false))
    (:`6`
      ;[1 1 1] S右
      (`SceneComponent.K2_AddLocalOffset` (`self.Cube1`) (0.0 0.0 0.0) false false)
      (`SceneComponent.K2_AddLocalOffset` (`self.Cube2`) (0.0 50.0 0.0) false false)
      (`SceneComponent.K2_AddLocalOffset` (`self.Cube3`) (0.0 100.0 0.0) false false)
      (`SceneComponent.K2_AddLocalOffset` (`self.Cube4`) (0.0 50.0 50.0) false false))))