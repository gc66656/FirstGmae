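; Falling Tetris piece that takes one of seven random four-cube shapes and matching glow colors in its construction script.
; A looping timer drops it one cell until a downward trace hits WorldStatic, then it spawns BP_singleBox per cube and a new BP_Tetromino, and destroys itself.
; Input moves or rotates it, reverting when box overlaps detect a collision; fast descent raises global time dilation.
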(event `InputAction|RotateBlock`
  (params (Key :type "Key Structure"))
  (:`Pressed`
    (`self.TryRotate`)))

(event `InputAction|MoveBlockLeft`
  (params (Key :type "Key Structure"))
  (:`Pressed`
    (`self.TryMove` -50.0)))

(event `InputAction|MoveBlockRight`
  (params (Key :type "Key Structure"))
  (:`Pressed`
    (`self.TryMove` 50.0)))

(event `InputAction|SpeedBlockDescent`
  (params (Key :type "Key Structure"))
  (:`Pressed`
    (`GameplayStatics.SetGlobalTimeDilation` 10.0))
  (:`Released`
    (`GameplayStatics.SetGlobalTimeDilation` 1.0)))

(event `self.ReceiveBeginPlay`
  (bind _returnvalue (`KismetSystemLibrary.K2_SetTimerDelegate` (delegate `Drop`) (`self.DropSpeed`) true))
  (set `self.DropTimer` _returnvalue))

(event `Drop`
  (set `self.CanDrop` true)
  (for _array_element (`SceneComponent.GetChildrenComponents` (`self.DefaultSceneRoot`) false)
    (bind _returnvalue (`SceneComponent.K2_GetComponentLocation` _array_element))
    (bind (_outhit _returnvalue_2) (`KismetSystemLibrary.LineTraceSingleForObjects` _returnvalue (+ _returnvalue (0.0 0.0 -50.0)) (`|MakeArray` "ObjectTypeQuery1" :!type "EObjectTypeQuery Enum")))
    (if _returnvalue_2
      (`/Engine/EditorBlueprintResources/StandardMacros.DoOnce` false
        (:`Completed`
          (set `self.CanDrop` false)
          (`KismetSystemLibrary.K2_ClearAndInvalidateTimerHandle` (`self.DropTimer`))))))
  (if (`self.CanDrop`)
    (`self.K2_AddActorWorldOffset` (0.0 0.0 -50.0))
    (else
      (for _array_element_2 (`SceneComponent.GetChildrenComponents` (`self.DefaultSceneRoot`) false)
        (`|SpawnActorFromClass` "/Game/BP/BP_singleBox.BP_singleBox_C" (`KismetMathLibrary.MakeTransform` (`SceneComponent.K2_GetComponentLocation` _array_element_2)) "Undefined" "OverrideRootScale" null (`self.color`) null))
      (`|SpawnActorFromClass` "BP_Tetromino_C" (`KismetMathLibrary.MakeTransform` (0.0 25.0 1000.0)) "Undefined" "OverrideRootScale" null null)
      (`self.K2_DestroyActor`))))

(fn `TryMove`
  (params (MoveAmount :type "Float (double-precision)"))
  (`self.K2_AddActorWorldOffset` (`KismetMathLibrary.MakeVector` 0.0 MoveAmount))
  (for _array_element (`SceneComponent.GetChildrenComponents` (`self.DefaultSceneRoot`) false)
    (bind (_outactors _returnvalue) (`KismetSystemLibrary.BoxOverlapActors` (`SceneComponent.K2_GetComponentLocation` _array_element) (20.0 20.0 20.0) (`|MakeArray` "ObjectTypeQuery1" :!type "EObjectTypeQuery Enum")))
    (if _returnvalue
      (`self.K2_AddActorWorldOffset` (`KismetMathLibrary.MakeVector` 0.0 (- 0.0 (`local.MoveAmount`))))
      (break))))

(fn `TryRotate`
  (`SceneComponent.K2_AddLocalRotation` (`self.DefaultSceneRoot`) (struct :`Roll` 90.0) false false)
  (for _array_element (`SceneComponent.GetChildrenComponents` (`self.DefaultSceneRoot`) false)
    (bind (_outactors _returnvalue) (`KismetSystemLibrary.BoxOverlapActors` (`SceneComponent.K2_GetComponentLocation` _array_element) (20.0 20.0 20.0) (`|MakeArray` "ObjectTypeQuery1" :!type "EObjectTypeQuery Enum")))
    (if _returnvalue
      (`SceneComponent.K2_AddLocalRotation` (`self.DefaultSceneRoot`) (struct :`Roll` -90.0) false false)
      (break))))

(fn `UserConstructionScript`
  (switch `int` (`KismetMathLibrary.RandomIntegerInRange` 0 6)
    (:`0`
      ;[1 1 1] I
      (`SceneComponent.K2_AddLocalOffset` (`self.cube1`) (0.0 0.0 0.0) false false)
      (`SceneComponent.K2_AddLocalOffset` (`self.cube2`) (0.0 50.0 0.0) false false)
      (`SceneComponent.K2_AddLocalOffset` (`self.cube3`) (0.0 100.0 0.0) false false)
      (`SceneComponent.K2_AddLocalOffset` (`self.cube4`) (0.0 150.0 0.0) false false)
      (set `self.color` (struct :`R` 1.0 :`A` 1.0)))
    (:`1`
      ;[1 1 1] I
      (`SceneComponent.K2_AddLocalOffset` (`self.cube1`) (0.0 0.0 0.0) false false)
      (`SceneComponent.K2_AddLocalOffset` (`self.cube2`) (0.0 50.0 0.0) false false)
      (`SceneComponent.K2_AddLocalOffset` (`self.cube3`) (0.0 100.0 0.0) false false)
      (`SceneComponent.K2_AddLocalOffset` (`self.cube4`) (0.0 0.0 50.0) false false)
      (set `self.color` (struct :`R` 1.0 :`B` 0.77448 :`A` 1.0)))
    (:`2`
      ;[1 1 1] I
      (`SceneComponent.K2_AddLocalOffset` (`self.cube1`) (0.0 0.0 0.0) false false)
      (`SceneComponent.K2_AddLocalOffset` (`self.cube2`) (0.0 50.0 0.0) false false)
      (`SceneComponent.K2_AddLocalOffset` (`self.cube3`) (0.0 100.0 0.0) false false)
      (`SceneComponent.K2_AddLocalOffset` (`self.cube4`) (0.0 100.0 50.0) false false)
      (set `self.color` (struct :`R` 1.0 :`G` 0.658564 :`A` 1.0)))
    (:`3`
      ;[1 1 1] o
      (`SceneComponent.K2_AddLocalOffset` (`self.cube1`) (0.0 0.0 0.0) false false)
      (`SceneComponent.K2_AddLocalOffset` (`self.cube2`) (0.0 50.0 0.0) false false)
      (`SceneComponent.K2_AddLocalOffset` (`self.cube3`) (0.0 0.0 50.0) false false)
      (`SceneComponent.K2_AddLocalOffset` (`self.cube4`) (0.0 50.0 50.0) false false)
      (set `self.color` (struct :`G` 1.0 :`B` 0.059249 :`A` 1.0)))
    (:`4`
      ;[1 1 1] S
      (`SceneComponent.K2_AddLocalOffset` (`self.cube1`) (0.0 0.0 0.0) false false)
      (`SceneComponent.K2_AddLocalOffset` (`self.cube2`) (0.0 50.0 0.0) false false)
      (`SceneComponent.K2_AddLocalOffset` (`self.cube3`) (0.0 50.0 50.0) false false)
      (`SceneComponent.K2_AddLocalOffset` (`self.cube4`) (0.0 100.0 50.0) false false)
      (set `self.color` (struct :`R` 1.0 :`G` 0.994607 :`A` 1.0)))
    (:`5`
      ;[1 1 1] Z
      (`SceneComponent.K2_AddLocalOffset` (`self.cube1`) (0.0 0.0 0.0) false false)
      (`SceneComponent.K2_AddLocalOffset` (`self.cube2`) (0.0 50.0 0.0) false false)
      (`SceneComponent.K2_AddLocalOffset` (`self.cube3`) (0.0 -50.0 50.0) false false)
      (`SceneComponent.K2_AddLocalOffset` (`self.cube4`) (0.0 0.0 50.0) false false)
      (set `self.color` (struct :`G` 0.986859 :`B` 1.0 :`A` 1.0)))
    (:`6`
      ;[1 1 1] T
      (`SceneComponent.K2_AddLocalOffset` (`self.cube1`) (0.0 0.0 0.0) false false)
      (`SceneComponent.K2_AddLocalOffset` (`self.cube2`) (0.0 50.0 0.0) false false)
      (`SceneComponent.K2_AddLocalOffset` (`self.cube3`) (0.0 100.0 0.0) false false)
      (`SceneComponent.K2_AddLocalOffset` (`self.cube4`) (0.0 50.0 50.0) false false)
      (set `self.color` (struct :`G` 0.139654 :`B` 1.0 :`A` 1.0))))
  (`MeshComponent.SetVectorParameterValueOnMaterials` (`self.cube1`) "GlowColor" (`KismetMathLibrary.Conv_LinearColorToVector` (`self.color`)))
  (`MeshComponent.SetVectorParameterValueOnMaterials` (`self.cube2`) "GlowColor" (`KismetMathLibrary.Conv_LinearColorToVector` (`self.color`)))
  (`MeshComponent.SetVectorParameterValueOnMaterials` (`self.cube3`) "GlowColor" (`KismetMathLibrary.Conv_LinearColorToVector` (`self.color`)))
  (`MeshComponent.SetVectorParameterValueOnMaterials` (`self.cube4`) "GlowColor" (`KismetMathLibrary.Conv_LinearColorToVector` (`self.color`))))