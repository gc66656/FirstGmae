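; BP_singleBox is a colored box actor that can drop one step down, apparently as a piece in a block-based game.
; BeginPlay applies its Color to the box materials' GlowColor parameter.
; While CanDrop is set, Tick traces a short line downward for WorldStatic objects and updates IsMoving.
; If clear, a DoOnce with no visible reset offsets the actor down without sweep and clears CanDrop.
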(event `self.ReceiveBeginPlay`
  (`MeshComponent.SetVectorParameterValueOnMaterials` (`self.box`) "GlowColor" (`KismetMathLibrary.Conv_LinearColorToVector` (`self.color`))))

(event `self.ReceiveTick`
  (params (DeltaSeconds :type "Float (single-precision)"))
  (bind _returnvalue (`SceneComponent.K2_GetComponentLocation` (`self.DefaultSceneRoot`)))
  (if (`self.CanDrop`)
    (bind (_outhit _returnvalue_2) (`KismetSystemLibrary.LineTraceSingleForObjects` _returnvalue (+ _returnvalue (0.0 0.0 -26.0)) (`|MakeArray` "ObjectTypeQuery1" :!type "EObjectTypeQuery Enum")))
    (if _returnvalue_2
      (set `self.isMoving` false)
      (else
        (set `self.isMoving` true)
        (`/Engine/EditorBlueprintResources/StandardMacros.DoOnce` false
          (:`Completed`
            (`self.K2_AddActorWorldOffset` (0.0 0.0 -50.0))
            (set `self.CanDrop` false)))))))

(fn `UserConstructionScript`)