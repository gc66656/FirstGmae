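; BP_checklines is a line-checker actor that clears a full row of BP_singleBox blocks in what appears to be a Tetris-style game.
; Every Tick, it counts non-moving boxes overlapping its Box component and flags the row full when the count reaches ten.
; A full row spawns an explosion at each overlapping box, sets CanDrop on all BP_singleBox actors in the level, and destroys the overlapping boxes.
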(event `self.ReceiveTick`
  (params (DeltaSeconds :type "Float (single-precision)"))
  (`|ExecutionSequence`
    (:`then_0`
      (bind _output_get (set `self.Overlapping Actors` (`PrimitiveComponent.GetOverlappingActors` (`self.Box`) "/Game/BP/BP_singleBox.BP_singleBox_C")))
      (for _array_element _output_get
        (bind _asbp_single_box (cast `/Game/BP/BP_singleBox` _array_element))
        (if (not (`/Game/BP/BP_singleBox.isMoving` _asbp_single_box))
          (`/Engine/EditorBlueprintResources/StandardMacros.IncrementInt` (`self.Length`)
            (:`  `
              (if (== (`self.Length`) 10)
                (set `self.Full` true))))))
      (set `self.Length` 0))
    (:`then_1`
      (if (`self.Full`)
        (for _array_element_2 (`self.Overlapping Actors`)
          ;[1 1 1] 消除逻辑
          (`GameplayStatics.SpawnEmitterAtLocation` "/Game/StarterContent/Particles/P_Explosion.P_Explosion" (`self.K2_GetActorLocation` _array_element_2))
          (set `self.Length` 0)
          (set `self.Full` false)
          (`|ExecutionSequence`
            (:`then_0`
              (bind _outactors (`GameplayStatics.GetAllActorsOfClass` "/Game/BP/BP_singleBox.BP_singleBox_C"))
              (for _array_element_3 _outactors
                (bind _asbp_single_box_2 (cast `/Game/BP/BP_singleBox` _array_element_3))
                (set `/Game/BP/BP_singleBox.CanDrop` true _asbp_single_box_2)))
            (:`then_1`
              (`self.K2_DestroyActor` _array_element_2))))))))

(fn `UserConstructionScript`)